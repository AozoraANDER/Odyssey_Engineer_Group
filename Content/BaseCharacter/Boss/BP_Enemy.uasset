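; Boss enemy character that runs BT_Enemy and stores the player character as its blackboard target.
; Ready plays a random equip montage, then flags ReadyToFight; AIAttack steps through a four-montage combo, with roughly a one-in-ten chance to dodge instead.
; Notify events reset attack state and combo index, while non-heavy damage plays a hit reaction and clears the attack lock.
; GetLocked passes lock-on state to its lock icon widget.
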(event Custom|ResetAttackMontage
  ;[1 1 1] Receive Notify
  (Variables|Default|SetAttackMontage false))

(event Custom|EndingCombo
  ;[1 1 1] Receive Notify
  (Variables|Default|SetAttackIndex 0))

(event Custom|AIAttack
  ;[1 1 1] Attack
  (if (not (or (Variables|Default|GetAttackMontage) (Variables|Default|GetHitMontage)))
    (if (== (Variables|Default|GetAttackIndex) 4)
      (Variables|Default|SetAttackIndex 0))
    (Variables|Default|SetAttackMontage true)
    (if (CallFunction|RandomChecker 10)
      (Animation|Montage|MontagePlay (Components|SkeletalMesh|GetAnimInstance (Variables|Character|GetMesh)) (Utilities|Array|Get(acopy) (Variables|Default|GetAttackMontages) (Variables|Default|GetAttackIndex)) 1.0 "MontageLength" 0.0 true)
      (if (== (Variables|Default|GetAttackIndex) 3)
        (Utilities|FlowControl|Delay 2.0))
      (Math|Integer|IncrementInt (Variables|Default|GetAttackIndex))
      (else
        (bind _returnvalue (Animation|Montage|MontagePlay (Components|SkeletalMesh|GetAnimInstance (Variables|Character|GetMesh)) (Utilities|Array|Get(acopy) (Variables|Default|GetDodgeMontages) (Math|Random|RandomIntegerinRange 0 3)) 1.0 "MontageLength" 0.0 true))
        (Utilities|FlowControl|Delay (- _returnvalue 0.3))
        (Variables|Default|SetAttackMontage false)))))

(event EventBeginPlay
  ;[1 1 1] Initialize
  (AI|RunBehaviorTree (AI|GetAIController self) "/Game/BaseCharacter/Boss/BT_Enemy.BT_Enemy")
  (AI|Components|Blackboard|SetValueasBool (AI|GetBlackboard 0) (Utilities|Name|MakeLiteralName "IfAllowFight") false)
  (bind _returnvalue (Actor|GetActorOfClass "/Game/BaseCharacter/BP_BaseCharacter.BP_BaseCharacter_C"))
  (bind _output_get (Variables|Default|SetTarget _returnvalue))
  (AI|Components|Blackboard|SetValueasObject (AI|GetBlackboard 0) (Utilities|Name|MakeLiteralName "Target") _output_get))

(event Game|Damage|EventAnyDamage
  (params (Damage :type Float%20%28single-precision%29) (DamageType :type Damage%20Type%20Object%20Reference) (InstigatedBy :type Controller%20Object%20Reference) (DamageCauser :type Actor%20Object%20Reference))
  (if (!= DamageType "/Game/BaseCharacter/BP_Damage_Heavy.BP_Damage_Heavy")
    (if (not (Variables|Default|GetHitMontage))
      (Variables|Default|SetHitMontage true)
      (Animation|Montage|MontagePlay (Components|SkeletalMesh|GetAnimInstance (Variables|Character|GetMesh)) "/Game/GhostSamurai_Bundle/GhostSamurai/Katana/Apose/Hit/Root/GhostSamurai_APose_Hit_F_Root_Montage.GhostSamurai_APose_Hit_F_Root_Montage" 1.0 "MontageLength" 0.0 true)
      (Variables|Default|SetHitMontage false)
      (Variables|Default|SetAttackMontage false))))

(event EventReady
  ;[1 1 1] Fight Ready Now
  (Variables|Default|SetEquip true)
  (bind _returnvalue (Animation|Montage|MontagePlay (Components|SkeletalMesh|GetAnimInstance (Variables|Character|GetMesh)) (Utilities|Select :Index (Math|Random|RandomIntegerinRange 0 1) :Option%200 "/Game/GhostSamurai_Bundle/GhostSamurai/Katana/Common/Root/GhostSamurai_APose_Equip01_Root_Montage.GhostSamurai_APose_Equip01_Root_Montage" :Option%201 "/Game/GhostSamurai_Bundle/GhostSamurai/Katana/Common/Root/GhostSamurai_APose_Equip02_Root_Montage.GhostSamurai_APose_Equip02_Root_Montage") 1.0 "MontageLength" 0.0 true))
  (Utilities|FlowControl|Delay (- _returnvalue 0.3))
  (AI|Components|Blackboard|SetValueasBool (AI|GetBlackboard self) (Utilities|Name|MakeLiteralName "ReadyToFight") true))

(fn ConstructionScript)

(fn GetLocked
  (params (IfLocked :type Boolean))
  (bind _aswbp_lock_icon (Utilities|Casting|CastToWBP_LockIcon (UserInterface|GetWidget (Variables|Default|GetWidget))))
  (Variables|/Game/BaseCharacter/Lock/WBP_LockIcon.WBP_LockIcon_C|SetIfLocked _aswbp_lock_icon IfLocked))

(fn RandomChecker
  (params (Chance :type Integer))
  (return (> (Math|Random|RandomIntegerinRange 1 100) Chance)))