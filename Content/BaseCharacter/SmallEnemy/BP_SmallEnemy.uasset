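; Small melee enemy character driven by BT_SmallEnemy, with the player character set as its blackboard target.
; When the player enters its box, it plays an equip montage and flags ReadyToFight.
; AIAttack usually advances a montage combo, occasionally dodging instead, while AttackSphere applies damage through a forward sphere trace.
; Non-heavy damage triggers hit reactions, death ragdolls then destroys it, and GetLocked updates its lock-on icon.
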(event OnComponentBeginOverlap(Box)
  (params (OverlappedComponent :type Primitive%20Component%20Object%20Reference) (OtherActor :type Actor%20Object%20Reference) (OtherComp :type Primitive%20Component%20Object%20Reference) (OtherBodyIndex :type Integer) (bFromSweep :type Boolean) (SweepResult :type Hit%20Result%20Structure%20%28by%20ref%29))
  (if (== OtherActor (Game|GetPlayerCharacter 0))
    (CallFunction|Ready)))

(event Custom|ResetAttackMontage
  ;[1 1 1] Receive Notify
  (Variables|Default|SetAttackMontage false))

(event Custom|EndingCombo
  ;[1 1 1] Receive Notify
  (Variables|Default|SetAttackIndex 0))

(event Custom|AIAttack
  ;[1 1 1] Attack
  (if (not (or (Variables|Default|GetAttackMontage) (Variables|Default|GetHitMontage)))
    (if (== (Variables|Default|GetAttackIndex) 4)
      (Variables|Default|SetAttackIndex 0))
    (Variables|Default|SetAttackMontage true)
    (if (CallFunction|RandomChecker 10)
      (Animation|Montage|MontagePlay (Components|SkeletalMesh|GetAnimInstance (Variables|Character|GetMesh)) (Utilities|Array|Get(acopy) (Variables|Default|GetAttackMontages) (Variables|Default|GetAttackIndex)) 1.0 "MontageLength" 0.0 true)
      (if (== (Variables|Default|GetAttackIndex) 3)
        (Utilities|FlowControl|Delay 2.0))
      (Math|Integer|IncrementInt (Variables|Default|GetAttackIndex))
      (else
        (bind _returnvalue (Animation|Montage|MontagePlay (Components|SkeletalMesh|GetAnimInstance (Variables|Character|GetMesh)) (Utilities|Array|Get(acopy) (Variables|Default|GetDodgeMontages) (Math|Random|RandomIntegerinRange 0 3)) 1.0 "MontageLength" 0.0 true))
        (Utilities|FlowControl|Delay (- _returnvalue 0.2))
        (Variables|Default|SetAttackMontage false)))))

(event Custom|AttackSphere
  (bind _attackposition (Variables|Default|GetAttackPosition))
  (bind _returnvalue (Transformation|GetWorldLocation _attackposition))
  (bind (_outhits _returnvalue_2) (Collision|MultiSphereTraceByChannel _returnvalue (+ _returnvalue (* (Math|Vector|GetForwardVector _attackposition) 5e+01)) 5e+01 "TraceTypeQuery1" false 0 "None"))
  (if _returnvalue_2
    (for _array_element _outhits
      (Utilities|FlowControl|DoOnce false :!label _label
        (:Completed
          (Game|Damage|ApplyDamage (.HitActor (Collision|BreakHitResult _array_element)) 15.0 0 self "/Game/BaseCharacter/BP_Damage_Basic.BP_Damage_Basic_C")
          (Utilities|FlowControl|Delay 0.3)
          (goto _label Reset))))))

(event EventBeginPlay
  ;[1 1 1] Initialize
  (AI|RunBehaviorTree (AI|GetAIController self) "/Game/BaseCharacter/SmallEnemy/BT_SmallEnemy.BT_SmallEnemy")
  (AI|Components|Blackboard|SetValueasBool (AI|GetBlackboard 0) (Utilities|Name|MakeLiteralName "IfAllowFight") false)
  (bind _returnvalue (Actor|GetActorOfClass "/Game/BaseCharacter/BP_BaseCharacter.BP_BaseCharacter_C"))
  (bind _output_get (Variables|Default|SetTarget _returnvalue))
  (AI|Components|Blackboard|SetValueasObject (AI|GetBlackboard 0) (Utilities|Name|MakeLiteralName "Target") _output_get))

(event Game|Damage|EventAnyDamage
  (params (Damage :type Float%20%28single-precision%29) (DamageType :type Damage%20Type%20Object%20Reference) (InstigatedBy :type Controller%20Object%20Reference) (DamageCauser :type Actor%20Object%20Reference))
  (bind _output_get (Variables|Default|SetHealth (- (Variables|Default|GetHealth) Damage)))
  (if (<= _output_get 0.0)
    (Utilities|FlowControl|DoOnce false
      (:Completed
        (Physics|SetSimulatePhysics (Variables|Character|GetMesh) true)
        (Variables|Default|SetEquip false)
        (Utilities|FlowControl|Delay 6.0)
        (Actor|DestroyActor)))
    (elif (!= DamageType "/Game/BaseCharacter/BP_Damage_Heavy.BP_Damage_Heavy")
      (if (not (Variables|Default|GetHitMontage))
        (Variables|Default|SetHitMontage true)
        (Animation|Montage|MontagePlay (Components|SkeletalMesh|GetAnimInstance (Variables|Character|GetMesh)) "/Game/GhostSamurai_Bundle/GhostSamurai/Katana/Apose/Hit/Root/GhostSamurai_APose_Hit_F_Root_Montage.GhostSamurai_APose_Hit_F_Root_Montage" 0.6 "MontageLength" 0.0 true)
        (Variables|Default|SetHitMontage false)
        (Variables|Default|SetAttackMontage false)))))

(event EventGetLocked
  (params (IfLocked :type Boolean))
  (bind _aswbp_lock_icon (Utilities|Casting|CastToWBP_LockIcon (UserInterface|GetWidget (Variables|Default|GetWidget))))
  (Variables|/Game/BaseCharacter/Lock/WBP_LockIcon.WBP_LockIcon_C|SetIfLocked _aswbp_lock_icon IfLocked))

(event EventReady
  ;[1 1 1] Fight Ready Now
  (Variables|Default|SetEquip true)
  (bind _returnvalue (Animation|Montage|MontagePlay (Components|SkeletalMesh|GetAnimInstance (Variables|Character|GetMesh)) (Utilities|Select :Index (Math|Random|RandomIntegerinRange 0 1) :Option%200 "/Game/GhostSamurai_Bundle/GhostSamurai/Katana/Common/Root/GhostSamurai_APose_Equip01_Root_Montage.GhostSamurai_APose_Equip01_Root_Montage" :Option%201 "/Game/GhostSamurai_Bundle/GhostSamurai/Katana/Common/Root/GhostSamurai_APose_Equip02_Root_Montage.GhostSamurai_APose_Equip02_Root_Montage") 1.0 "MontageLength" 0.0 true))
  (Utilities|FlowControl|Delay (- _returnvalue 0.3))
  (AI|Components|Blackboard|SetValueasBool (AI|GetBlackboard self) (Utilities|Name|MakeLiteralName "ReadyToFight") true))

(fn ConstructionScript)

(fn GetLocked
  (params (IfLocked :type Boolean))
  (bind _aswbp_lock_icon (Utilities|Casting|CastToWBP_LockIcon (UserInterface|GetWidget (Variables|Default|GetWidget))))
  (Variables|/Game/BaseCharacter/Lock/WBP_LockIcon.WBP_LockIcon_C|SetIfLocked _aswbp_lock_icon IfLocked))

(fn RandomChecker
  (params (Chance :type Integer))
  (return (> (Math|Random|RandomIntegerinRange 1 100) Chance)))