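; Giant double door actor whose OpenDoor event slides the Left and Right components to open positions.
; A timeline, gated by DoorOpened (not set in these graphs), lerps each component from its current location by a scaled-down track value every update, so movement is incremental rather than a fixed start-to-end blend.
; When the timeline finishes, player controller 0 blends its view target to the passed-in Player.
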(event Custom|Open%20Door
  (params (Player :type Actor%20Object%20Reference))
  (if (not (Variables|Default|GetbDoorOpened))
    (bind _open_track (Timeline|Door%20Open%20T Play)
      (:Update
        (Utilities|FlowControl|Sequence
          (:then_0
            (Transformation|SetRelativeLocation (Variables|Default|GetLeft) (Math|Vector|Lerp(Vector) (Variables|/Script/Engine.SceneComponent|GetRelativeLocation (Variables|Default|GetLeft)) "0.000000,-350.000000,180.000000" (* _open_track 0.05)) false false))
          (:then_1
            (Transformation|SetRelativeLocation (Variables|Default|GetRight) (Math|Vector|Lerp(Vector) (Variables|/Script/Engine.SceneComponent|GetRelativeLocation (Variables|Default|GetRight)) "0.000000,390.000000,180.000000" (* _open_track 0.05)) false false))))
      (:Finished
        (Game|Player|SetViewTargetwithBlend (Game|GetPlayerController 0) Player 1.2 "VTBlend_Linear" 0.0 false)))))

(fn ConstructionScript)