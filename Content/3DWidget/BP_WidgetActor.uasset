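; BP_WidgetActor is an interactable actor that lets the player toggle a fixed camera view with mouse control, apparently for a 3D widget.
; Overlap on component R enables input while the player character is inside and disables it on exit.
; Pressing E flip-flops between blending to the camera actor tagged "A" with cursor and Game and UI input, and blending back to the character with game-only input.
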(event OnComponentBeginOverlap(r)
  (params (OverlappedComponent :type Primitive%20Component%20Object%20Reference) (OtherActor :type Actor%20Object%20Reference) (OtherComp :type Primitive%20Component%20Object%20Reference) (OtherBodyIndex :type Integer) (bFromSweep :type Boolean) (SweepResult :type Hit%20Result%20Structure%20%28by%20ref%29))
  (if (== OtherActor (Game|GetPlayerCharacter 0))
    (Input|EnableInput (Game|GetPlayerController 0))))

(event OnComponentEndOverlap(r)
  (params (OverlappedComponent :type Primitive%20Component%20Object%20Reference) (OtherActor :type Actor%20Object%20Reference) (OtherComp :type Primitive%20Component%20Object%20Reference) (OtherBodyIndex :type Integer))
  (if (== OtherActor (Game|GetPlayerCharacter 0))
    (Input|DisableInput (Game|GetPlayerController 0))))

(event EventBeginPlay)

(event Collision|EventActorBeginOverlap
  (params (OtherActor :type Actor%20Object%20Reference)))

(event EventTick
  (params (DeltaSeconds :type Float%20%28single-precision%29)))

(event Input|KeyboardEvents|E
  (params (Key :type Key%20Structure))
  (bind _returnvalue (Game|GetPlayerController 0))
  (bind _returnvalue_2 (Game|GetPlayerController 0))
  (:Pressed
    (Utilities|FlowControl|FlipFlop
      (:A
        (Variables|/Script/Engine.PlayerController|SetbShowMouseCursor _returnvalue true)
        (bind _outactors (Actor|GetAllActorswithTag "A"))
        (for _array_element _outactors
          (bind _ascamera_actor (Utilities|Casting|CastToCameraActor _array_element))
          (Game|Player|SetViewTargetwithBlend _returnvalue _ascamera_actor 1.0 "VTBlend_Linear" 0.0 false)
          (Input|SetInputModeGameandUI _returnvalue_2 0 "DoNotLock" true false)))
      (:B
        (Variables|/Script/Engine.PlayerController|SetbShowMouseCursor _returnvalue false)
        (Game|Player|SetViewTargetwithBlend _returnvalue (Game|GetPlayerCharacter 0) 1.0 "VTBlend_Linear" 0.0 false)
        (Input|SetInputModeGameOnly _returnvalue_2 false)))))

(fn ConstructionScript)