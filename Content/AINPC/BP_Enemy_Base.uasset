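; Base enemy AI character that patrols, wields a sword, attacks the player and drops an access card on death.
; Attack plays a montage, immediately damages the player if inside AttackSphere, then fires OnAttackEnd.
; Incoming damage, scaled a hundredfold, updates an initially hidden health widget; death triggers an explosion, a ground-traced card drop and destruction.
; Helper functions expose the patrol route, walk speed and health bar visibility.
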(event Custom|Attack
  (bind _returnvalue (Game|GetPlayerCharacter 0))
  (bind _asbp_base_character (Utilities|Casting|CastToBP_BaseCharacter (Game|GetPlayerCharacter 0)))
  (bind _newparam (Default|CheckIsAlive _asbp_base_character))
  (if _newparam
    (Animation|Montage|MontagePlay (Components|SkeletalMesh|GetAnimInstance (Variables|Character|GetMesh)) "/Game/AINPC/Montage_Attack.Montage_Attack" 1.0 "MontageLength" 0.0 true)
    (for _array_element (Collision|GetOverlappingActors (Variables|Default|GetAttackSphere) "/Game/BaseCharacter/BP_BaseCharacter.BP_BaseCharacter_C" :!class /Script/Engine.PrimitiveComponent)
      (if (== _array_element _returnvalue)
        (Game|Damage|ApplyDamage _returnvalue 2e+01 0 0)))
    (Default|CallOnAttackEnd)))

(event Custom|wieldSword
  (bind _returnvalue (Game|SpawnActorfromClass (Variables|Default|GetSword) (Transformation|GetActorTransform) "Undefined" "MultiplyWithRoot" 0 0))
  (Transformation|AttachComponentToComponent _returnvalue (Variables|Character|GetMesh) "hand_r_sword_socket" "SnapToTarget" "SnapToTarget" "SnapToTarget" true)
  (Variables|Default|SetIsWiedingSword true))

(event Custom|DropLoot
  (bind _returnvalue (Transformation|GetActorLocation))
  ;[1 1 1] Drop Access Card
  (bind _outhit (Collision|LineTraceByChannel _returnvalue (- _returnvalue "0.000000,0.000000,200.000000") "TraceTypeQuery1" false (Utilities|Array|MakeArray (Game|GetPlayerCharacter 0)) "None"))
  (Game|SpawnActorfromClass "/Game/Interactables/Access_Card/BP_AccessCard.BP_AccessCard_C" (Math|Transform|MakeTransform (.Location (Collision|BreakHitResult _outhit))) "Undefined" "MultiplyWithRoot" 0 0))

(event EventBeginPlay
  (Variables|Default|SetAnchor (Transformation|GetActorLocation))
  (Variables|Default|SetCurrentHealth 100)
  (Variables|/Script/Engine.CharacterMovementComponent|SetMaxWalkSpeed (Variables|Character|GetCharacterMovement) (Variables|Default|GetWalkSpeed))
  (bind _aswbp_enemy_health (Utilities|Casting|CastToWBP_EnemyHealth (UserInterface|GetUserWidgetObject (Variables|Default|GetWidget))))
  (bind _output_get (Variables|Default|SetWBP%20Health _aswbp_enemy_health))
  (Widget|SetVisibility _output_get "Hidden")
  (Variables|/Game/AINPC/EnemyWidget/WBP_EnemyHealth.WBP_EnemyHealth_C|SetCurrentHealth _output_get (Variables|Default|GetCurrentHealth))
  (Variables|/Game/AINPC/EnemyWidget/WBP_EnemyHealth.WBP_EnemyHealth_C|SetMaxHealth _output_get (Variables|Default|GetMaxHealth)))

(event Game|Damage|EventAnyDamage
  (params (Damage :type Float%20%28single-precision%29) (DamageType :type Damage%20Type%20Object%20Reference) (InstigatedBy :type Controller%20Object%20Reference) (DamageCauser :type Actor%20Object%20Reference))
  (Development|PrintText (Utilities|Text|ToText(Integer) (Variables|Default|GetCurrentHealth)))
  (bind _output_get (Variables|Default|SetCurrentHealth (- (Variables|Default|GetCurrentHealth) (* Damage 1e+02))))
  (Default|UpdateHealth (Variables|Default|GetWBP%20Health) (Math|Integer|Clamp(Integer) _output_get 0 (Variables|Default|GetMaxHealth)))
  (if (<= (Variables|Default|GetCurrentHealth) 0)
    (Effects|SpawnEmitterAttached "/Game/StarterContent/Particles/P_Explosion.P_Explosion" (Variables|Collision|GetCapsuleComponent) "None")
    (CallFunction|DropLoot)
    (Actor|DestroyActor)))

(fn ConstructionScript)

(fn SetMaxSpeed
  (params (speed :type Float%20%28double-precision%29))
  (Variables|/Script/Engine.CharacterMovementComponent|SetMaxWalkSpeed (Variables|Character|GetCharacterMovement) speed))

(fn SetEnemyHealthVisible
  (Widget|SetVisibility (Variables|Default|GetWBP%20Health) "Visible"))

(fn GetPatrolRoute
  (return (Variables|Default|GetPatrolRoute)))

(fn SetMovementSpeed
  (params (Speed :type E_MovementSpeed%20Enum :default "NewEnumerator0"))
  (bind _output_get (Variables|/Script/Engine.CharacterMovementComponent|SetMaxWalkSpeed (Variables|Character|GetCharacterMovement) (Utilities|Select :Index Speed :NewEnumerator0 0.0 :NewEnumerator1 1.5e+02 :NewEnumerator2 2e+02 :NewEnumerator3 4e+02)))
  (return _output_get))