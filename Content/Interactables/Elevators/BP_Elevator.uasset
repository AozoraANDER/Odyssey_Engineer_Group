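; BP_Elevator is an interactable elevator actor with timeline-driven movement for two floors and a "Press E" prompt.
; Interact accepts a BP_BaseCharacter and switches on a constant 0, so neither the Floor2 nor Floor3 case is reached as wired.
; Those timelines set the elevator's relative Z, and Floor2 resets the switch material after finishing.
; Box overlap events show and hide the prompt.
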(event EventInteract
  (params (Player :type Character%20Object%20Reference))
  (bind _elevator (Variables|Default|GetElevator))
  (bind _elevator_2 (Variables|Default|GetElevator))
  (bind _relativelocation (Variables|/Script/Engine.SceneComponent|GetRelativeLocation _elevator))
  (bind _relativelocation_2 (Variables|/Script/Engine.SceneComponent|GetRelativeLocation _elevator_2))
  (bind _asbp_base_character (Utilities|Casting|CastToBP_BaseCharacter Player))
  (switch int 0
    (:2
      (bind _z (Timeline|Floor%202 Play)
        (:Update
          (Transformation|SetRelativeLocation _elevator_2 (Math|Vector|MakeVector (.x _relativelocation_2) (.y _relativelocation_2) _z) false false))
        (:Finished
          (Utilities|FlowControl|Delay 0.2)
          (Rendering|Material|SetMaterial (Variables|Default|GetSwitch) 0 0))))
    (:3
      (bind _z_2 (Timeline|Floor%203 Play)
        (:Update
          (Transformation|SetRelativeLocation _elevator (Math|Vector|MakeVector (.x _relativelocation) (.y _relativelocation) _z_2) false false))))))

(fn ConstructionScript)

(event OnComponentBeginOverlap(Box)
  (params (OverlappedComponent :type Primitive%20Component%20Object%20Reference) (OtherActor :type Actor%20Object%20Reference) (OtherComp :type Primitive%20Component%20Object%20Reference) (OtherBodyIndex :type Integer) (bFromSweep :type Boolean) (SweepResult :type Hit%20Result%20Structure%20%28by%20ref%29))
  (Rendering|SetVisibility (Variables|Default|GetPress%20E) true false))

(event OnComponentEndOverlap(Box)
  (params (OverlappedComponent :type Primitive%20Component%20Object%20Reference) (OtherActor :type Actor%20Object%20Reference) (OtherComp :type Primitive%20Component%20Object%20Reference) (OtherBodyIndex :type Integer))
  (Rendering|SetVisibility (Variables|Default|GetPress%20E) false false))