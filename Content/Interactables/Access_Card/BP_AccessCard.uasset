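; BP_AccessCard is an interactable access card pickup that grants the player access card level 1.
; Overlapping its Box shows the PressE prompt, and leaving hides it.
; Interact casts the player to BP_BaseCharacter, plays a found sound at the Card's relative location, destroys the actor and sets the character's AccessCardLevel.
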(event EventInteract
  (params (Player :type Character%20Object%20Reference))
  (bind _asbp_base_character (Utilities|Casting|CastToBP_BaseCharacter Player))
  (Audio|PlaySoundatLocation "/Game/Interactables/Access_Card/Sound/ObjectFound.ObjectFound" (Variables|/Script/Engine.SceneComponent|GetRelativeLocation (Variables|Default|GetCard)) "0, 0, 0" 1.0 1.0 0.0 0 0 0 0)
  (Actor|DestroyActor)
  (Variables|/Game/BaseCharacter/BP_BaseCharacter.BP_BaseCharacter_C|SetAccess%20Card%20Level _asbp_base_character 1))

(fn ConstructionScript)

(event OnComponentBeginOverlap(Box)
  (params (OverlappedComponent :type Primitive%20Component%20Object%20Reference) (OtherActor :type Actor%20Object%20Reference) (OtherComp :type Primitive%20Component%20Object%20Reference) (OtherBodyIndex :type Integer) (bFromSweep :type Boolean) (SweepResult :type Hit%20Result%20Structure%20%28by%20ref%29))
  (Rendering|SetVisibility (Variables|Default|GetPress%20E) true false))

(event OnComponentEndOverlap(Box)
  (params (OverlappedComponent :type Primitive%20Component%20Object%20Reference) (OtherActor :type Actor%20Object%20Reference) (OtherComp :type Primitive%20Component%20Object%20Reference) (OtherBodyIndex :type Integer))
  (Rendering|SetVisibility (Variables|Default|GetPress%20E) false false))