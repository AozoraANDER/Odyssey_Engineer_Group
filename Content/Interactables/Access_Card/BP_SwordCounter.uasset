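; Interactable sword counter, built from Cube, Katana and Cylinder components, that stays hidden until revealed.
; BeginPlay disables actor collision and hides all three components; AppearCounter, which has no caller in this Blueprint, restores both.
; Box overlaps toggle the PressE prompt without filtering the overlapping actor.
; Interact only plays the ObjectFound sound for a BP_BaseCharacter, positioned at the Cube's relative rather than world location.
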(event EventBeginPlay
  (Collision|SetActorEnableCollision self false)
  (Rendering|SetVisibility (Variables|Default|GetCube) false false)
  (Rendering|SetVisibility (Variables|Default|Getkatana) false false)
  (Rendering|SetVisibility (Variables|Default|GetCylinder) false false))

(event EventInteract
  (params (Player :type Character%20Object%20Reference))
  (Utilities|Casting|CastToBP_BaseCharacter Player)
  (Audio|PlaySoundatLocation "/Game/Interactables/Access_Card/Sound/ObjectFound.ObjectFound" (Variables|/Script/Engine.SceneComponent|GetRelativeLocation (Variables|Default|GetCube)) "0, 0, 0" 1.0 1.0 0.0 0 0 0 0))

(fn ConstructionScript)

(fn AppearCounter
  (Collision|SetActorEnableCollision self true)
  (Rendering|SetVisibility (Variables|Default|GetCube) true false)
  (Rendering|SetVisibility (Variables|Default|Getkatana) true false)
  (Rendering|SetVisibility (Variables|Default|GetCylinder) true false))

(event OnComponentBeginOverlap(Box)
  (params (OverlappedComponent :type Primitive%20Component%20Object%20Reference) (OtherActor :type Actor%20Object%20Reference) (OtherComp :type Primitive%20Component%20Object%20Reference) (OtherBodyIndex :type Integer) (bFromSweep :type Boolean) (SweepResult :type Hit%20Result%20Structure%20%28by%20ref%29))
  (Rendering|SetVisibility (Variables|Default|GetPress%20E) true false))

(event OnComponentEndOverlap(Box)
  (params (OverlappedComponent :type Primitive%20Component%20Object%20Reference) (OtherActor :type Actor%20Object%20Reference) (OtherComp :type Primitive%20Component%20Object%20Reference) (OtherBodyIndex :type Integer))
  (Rendering|SetVisibility (Variables|Default|GetPress%20E) false false))