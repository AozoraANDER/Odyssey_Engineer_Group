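; BP_Button is a pressure-plate style button for the puzzle room that signals open and close as things enter and leave its collision.
; Begin overlap calls Open and lowers the Cube slightly with MoveComponentTo, while end overlap calls Close and raises it by the same offset.
; Overlaps are unfiltered and uncounted, and each move is relative to the Cube's current location.
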(event OnComponentBeginOverlap(Collision)
  (params (OverlappedComponent :type Primitive%20Component%20Object%20Reference) (OtherActor :type Actor%20Object%20Reference) (OtherComp :type Primitive%20Component%20Object%20Reference) (OtherBodyIndex :type Integer) (bFromSweep :type Boolean) (SweepResult :type Hit%20Result%20Structure%20%28by%20ref%29))
  (bind _cube (Variables|Default|GetCube))
  (Default|CallOpen)
  (Components|MoveComponentTo _cube (- (Variables|/Script/Engine.SceneComponent|GetRelativeLocation _cube) "0.000000,0.000000,10.000000") "0, 0, 0" false false 0.2 false))

(event OnComponentEndOverlap(Collision)
  (params (OverlappedComponent :type Primitive%20Component%20Object%20Reference) (OtherActor :type Actor%20Object%20Reference) (OtherComp :type Primitive%20Component%20Object%20Reference) (OtherBodyIndex :type Integer))
  (bind _cube (Variables|Default|GetCube))
  (Default|CallClose)
  (Components|MoveComponentTo _cube (+ (Variables|/Script/Engine.SceneComponent|GetRelativeLocation _cube) "0.000000,0.000000,10.000000") "0, 0, 0" false false 0.2 false))

(event EventBeginPlay)

(event Collision|EventActorBeginOverlap
  (params (OtherActor :type Actor%20Object%20Reference)))

(event EventTick
  (params (DeltaSeconds :type Float%20%28single-precision%29)))

(fn ConstructionScript)