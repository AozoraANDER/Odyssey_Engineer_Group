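; BP_Door is a puzzle-room door that slides open and closed in response to a BP_Button.
; On BeginPlay it finds a single BP_Button via GetActorOfClass and binds its Open and Close handlers to that button's events.
; Each handler uses MoveComponentTo to shift the static mesh along local Y by a fixed offset from its current relative location, rather than toward stored open and closed positions.
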(event Custom|Open
  (bind _staticmesh (Variables|Default|GetStaticMesh))
  (Components|MoveComponentTo _staticmesh (+ (Variables|/Script/Engine.SceneComponent|GetRelativeLocation _staticmesh) "0.000000,100.000000,0.000000") "0, 0, 0" false false 0.2 false))

(event Custom|Close
  (bind _staticmesh (Variables|Default|GetStaticMesh))
  (Components|MoveComponentTo _staticmesh (- (Variables|/Script/Engine.SceneComponent|GetRelativeLocation _staticmesh) "0.000000,100.000000,0.000000") "0, 0, 0" false false 0.2 false))

(event EventBeginPlay
  (bind _returnvalue (Actor|GetActorOfClass "/Game/ThirdPerson/Blueprints/BP_Button.BP_Button_C"))
  (bind _output_get (Variables|Default|SetButton _returnvalue))
  (EventDispatchers|BindEventtoOpen _output_get (delegate Custom|Open))
  (EventDispatchers|BindEventtoClose _output_get (delegate Custom|Close)))

(fn ConstructionScript)