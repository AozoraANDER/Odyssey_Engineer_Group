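; BP_Terminal is an interactable terminal that upgrades the player's access card when the correct password is entered.
; Box overlaps toggle the PressE prompt, and Interact opens a password widget with UI-only input and a visible cursor until the terminal is activated.
; On the widget's Completed callback, a correct result upgrades the card, plays a sound and locks out reuse.
; Either result then removes the widget and restores game input.
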(event Custom|Password%20Completed
  (bind _returnvalue (Game|GetPlayerController 0))
  (Utilities|FlowControl|Sequence
    (:then_0
      (if (Variables|/Game/UI/Password/PasswordWidget.PasswordWidget_C|Getcorrect (Variables|Default|GetpasswordWidget))
        (bind _asbp_base_character (Utilities|Casting|CastToBP_BaseCharacter (Variables|Default|GetPlayer)))
        (Default|UpgradeAccessCard _asbp_base_character)
        (Audio|PlaySound2D "/Game/Interactables/Access_Card/Sound/ObjectFound.ObjectFound" 1.0 1.0 0.0 0 0)
        (Variables|Default|SetbActivated true)))
    (:then_1
      (Input|SetInputModeGameOnly _returnvalue false)
      (Variables|/Script/Engine.PlayerController|SetbShowMouseCursor _returnvalue false)
      (Widget|RemovefromParent (Variables|Default|GetpasswordWidget)))))

(event EventInteract
  (params (Player :type Character%20Object%20Reference))
  (bind _returnvalue (Game|GetPlayerController 0))
  (Variables|Default|SetPlayer Player)
  (if (not (Variables|Default|GetbActivated))
    (Input|SetInputModeUIOnly _returnvalue 0 "DoNotLock" false)
    (Variables|/Script/Engine.PlayerController|SetbShowMouseCursor _returnvalue true)
    (bind _returnvalue_2 (UserInterface|CreateWidget "/Game/UI/Password/PasswordWidget.PasswordWidget_C"))
    (UserInterface|Viewport|AddtoViewport _returnvalue_2 0)
    (bind _output_get (Variables|Default|SetpasswordWidget _returnvalue_2))
    (EventDispatchers|AssignCompleted _output_get (delegate Custom|Password%20Completed))))

(fn ConstructionScript)

(event OnComponentBeginOverlap(Box)
  (params (OverlappedComponent :type Primitive%20Component%20Object%20Reference) (OtherActor :type Actor%20Object%20Reference) (OtherComp :type Primitive%20Component%20Object%20Reference) (OtherBodyIndex :type Integer) (bFromSweep :type Boolean) (SweepResult :type Hit%20Result%20Structure%20%28by%20ref%29))
  (Rendering|SetVisibility (Variables|Default|GetPress%20E) true false))

(event OnComponentEndOverlap(Box)
  (params (OverlappedComponent :type Primitive%20Component%20Object%20Reference) (OtherActor :type Actor%20Object%20Reference) (OtherComp :type Primitive%20Component%20Object%20Reference) (OtherBodyIndex :type Integer))
  (Rendering|SetVisibility (Variables|Default|GetPress%20E) false false))