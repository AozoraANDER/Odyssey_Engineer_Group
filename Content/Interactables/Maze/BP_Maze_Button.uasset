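; Maze button interactable that slides its linked wall back and forth when interacted with.
; Interact switches on the wall's color (Red, Green or White), then plays or reverses that color's timeline based on the Activated flag, which flips when the timeline finishes.
; Timeline values set absolute world position on one axis: X for red and white walls, Y for green.
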(event EventInteract
  (params (Player :type Character%20Object%20Reference))
  (switch string (Variables|/Game/Interactables/Maze/BP_MazeWall.BP_MazeWall_C|GetColor (Variables|Default|GetLinked%20Wall))
    (:Red
      (|RedActivated?
        (:true
          (bind _x (Timeline|Move%20Red Play)
            (:Update
              (|MoveRedWallLocation (.x _x)))
            (:Finished
              (CallFunction|FlipActivated))))
        (:false
          (Timeline|Move%20Red Reverse))))
    (:Green
      (|GreenActivated?
        (:true
          (bind _y_vector (Timeline|Move%20Green Play)
            (:Update
              (|MoveGreenWallLocation (.x_y _y_vector)))
            (:Finished
              (CallFunction|FlipActivated))))
        (:false
          (Timeline|Move%20Green Reverse))))
    (:White
      (|WhiteActivated?
        (:true
          (bind _x_2 (Timeline|Move%20White Play)
            (:Update
              (|MoveWhiteWallLocation (.x _x_2)))
            (:Finished
              (CallFunction|FlipActivated))))
        (:false
          (Timeline|Move%20White Reverse))))))

(fn ConstructionScript)

(fn FlipActivated
  (Variables|Default|SetActivated (not (Variables|Default|GetActivated))))