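; GiantDoor_Button_BP is an interactable button that opens its linked giant door for a player holding access card number 1.
; On Interact it casts to BP_BaseCharacter, checks the card, then opens the door once, guarded by the door's DoorOpened flag.
; Opening also blends the first player controller's view to the door.
; A Box overlap shows and hides the PressE prompt for any overlapping actor.
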(event EventInteract
  (params (Player :type Character%20Object%20Reference))
  (bind _linked_door (Variables|Default|GetLinked%20Door))
  (bind _asbp_base_character (Utilities|Casting|CastToBP_BaseCharacter Player))
  (if (== (Default|GetAccessCardNumber _asbp_base_character) 1)
    (if (not (Variables|/Game/Interactables/Doors/GiantDoor_BP.GiantDoor_BP_C|GetbDoorOpened _linked_door))
      (Default|OpenDoor _linked_door Player)
      (Game|Player|SetViewTargetwithBlend (Game|GetPlayerController 0) _linked_door 0.7 "VTBlend_Linear" 0.0 false)
      (Variables|/Game/Interactables/Doors/GiantDoor_BP.GiantDoor_BP_C|SetbDoorOpened _linked_door true))))

(fn ConstructionScript)

(event OnComponentBeginOverlap(Box)
  (params (OverlappedComponent :type Primitive%20Component%20Object%20Reference) (OtherActor :type Actor%20Object%20Reference) (OtherComp :type Primitive%20Component%20Object%20Reference) (OtherBodyIndex :type Integer) (bFromSweep :type Boolean) (SweepResult :type Hit%20Result%20Structure%20%28by%20ref%29))
  (Rendering|SetVisibility (Variables|Default|GetPressE) true false))

(event OnComponentEndOverlap(Box)
  (params (OverlappedComponent :type Primitive%20Component%20Object%20Reference) (OtherActor :type Actor%20Object%20Reference) (OtherComp :type Primitive%20Component%20Object%20Reference) (OtherBodyIndex :type Integer))
  (Rendering|SetVisibility (Variables|Default|GetPressE) false false))