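; BP_ShaderSwitch switches the level between realistic and toon looks from its construction script, based on IfReality.
; It toggles in-game visibility of BP_StylizedSky and Ultra_Dynamic_Sky, keeping Ultra_Dynamic_Weather visible in both.
; It flips Unbound on PostProcessVolumes tagged Toon and Bloom.
; All changes run inside the Bloom loop, and the empty Toon loop leaves only its last element affected.
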(fn ConstructionScript
  ;[1 1 1] Change shader
  (if (Variables|Default|GetIfReality)
    (Utilities|FlowControl|Sequence
      (:then_0
        (bind _outactors (Actor|GetAllActorsOfClasswithTag "/Script/Engine.PostProcessVolume" "Toon"))
        (for _array_element _outactors
          _))
      (:then_1
        (bind _returnvalue (Actor|GetActorOfClass "/Game/SoStylized/Environment/Sky/BP_StylizedSky.BP_StylizedSky_C")))
      (:then_2
        (bind _returnvalue_2 (Actor|GetActorOfClass "/Game/UltraDynamicSky/Blueprints/Ultra_Dynamic_Sky.Ultra_Dynamic_Sky_C")))
      (:then_3
        (bind _returnvalue_3 (Actor|GetActorOfClass "/Game/UltraDynamicSky/Blueprints/Ultra_Dynamic_Weather.Ultra_Dynamic_Weather_C")))
      (:then_4
        (bind _outactors_2 (Actor|GetAllActorsOfClasswithTag "/Script/Engine.PostProcessVolume" "Bloom"))
        (for _array_element_2 _outactors_2
          (Rendering|SetActorHiddenInGame _returnvalue true)
          (Rendering|SetActorHiddenInGame _returnvalue_2 false)
          (Variables|/Script/Engine.PostProcessVolume|SetbUnbound _array_element false)
          (Variables|/Script/Engine.PostProcessVolume|SetbUnbound _array_element_2 true))))
    (else
      (Utilities|FlowControl|Sequence
        (:then_0
          (bind _outactors_3 (Actor|GetAllActorsOfClasswithTag "/Script/Engine.PostProcessVolume" "Toon"))
          (for _array_element_3 _outactors_3
            _))
        (:then_1
          (bind _returnvalue_4 (Actor|GetActorOfClass "/Game/SoStylized/Environment/Sky/BP_StylizedSky.BP_StylizedSky_C")))
        (:then_2
          (bind _returnvalue_5 (Actor|GetActorOfClass "/Game/UltraDynamicSky/Blueprints/Ultra_Dynamic_Sky.Ultra_Dynamic_Sky_C")))
        (:then_3
          (bind _returnvalue_6 (Actor|GetActorOfClass "/Game/UltraDynamicSky/Blueprints/Ultra_Dynamic_Weather.Ultra_Dynamic_Weather_C")))
        (:then_4
          (bind _outactors_4 (Actor|GetAllActorsOfClasswithTag "/Script/Engine.PostProcessVolume" "Bloom"))
          (for _array_element_4 _outactors_4
            (Rendering|SetActorHiddenInGame _returnvalue_4 false)
            (Rendering|SetActorHiddenInGame _returnvalue_5 true)
            (Variables|/Script/Engine.PostProcessVolume|SetbUnbound _array_element_3 true)
            (Variables|/Script/Engine.PostProcessVolume|SetbUnbound _array_element_4 false)))))))