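; Interactable lift that travels one floor per use, reversing direction at the top and bottom.
; Floors are all BP_TargetPoint actors, matched by Index, and timelines lerp the lift between their locations.
; A box overlap toggles the player's interact prompt, and a DoOnce blocks Interact until the move finishes.
; A separate Callback event returns the lift to floor zero and resets its direction to up.
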(event OnComponentBeginOverlap(Box)
  (params (OverlappedComponent :type Primitive%20Component%20Object%20Reference) (OtherActor :type Actor%20Object%20Reference) (OtherComp :type Primitive%20Component%20Object%20Reference) (OtherBodyIndex :type Integer) (bFromSweep :type Boolean) (SweepResult :type Hit%20Result%20Structure%20%28by%20ref%29))
  (bind _returnvalue (Game|GetPlayerCharacter 0))
  (if (== OtherActor _returnvalue)
    (Class|BIPlayerInterface|SetInteractableState(Message) _returnvalue true (Variables|Default|GetTxt_Action))))

(event OnComponentEndOverlap(Box)
  (params (OverlappedComponent :type Primitive%20Component%20Object%20Reference) (OtherActor :type Actor%20Object%20Reference) (OtherComp :type Primitive%20Component%20Object%20Reference) (OtherBodyIndex :type Integer))
  (bind _returnvalue (Game|GetPlayerCharacter 0))
  (if (== _returnvalue OtherActor)
    (Class|BIPlayerInterface|SetInteractableState(Message) _returnvalue false (Variables|Default|GetTxt_Action))))

(event Custom|MoveLift
  (bind _self self)
  (bind _floors (Variables|Default|GetFloors))
  (if (Variables|Default|Getb_Is_Up)
    (if (== (+ (Variables|Default|GetCurrentFloor) 1) (Utilities|Array|Length _floors))
      (Variables|Default|Setb_Is_Up false)
      (CallFunction|MoveLift)
      (else
        (bind _output_get (Variables|Default|SetCurrent (Transformation|GetActorLocation _self)))
        (for _array_element _floors
          (if (== (Variables|/Game/Lift/BP_TargetPoint.BP_TargetPoint_C|GetIndex _array_element) (+ (Variables|Default|GetCurrentFloor) 1))
            (bind _output_get_2 (Variables|Default|SetTarget (Transformation|GetActorLocation _array_element)))))
        (bind _alpha (Timeline|Alpha PlayFromStart)
          (:Update
            (Transformation|SetActorLocation (Math|Vector|Lerp(Vector) _output_get _output_get_2 _alpha) false false))
          (:Finished
            (Variables|Default|SetCurrentFloor (+ (Variables|Default|GetCurrentFloor) 1))
            (Development|PrintString (Utilities|String|Append "Current Floor is:" (Utilities|String|ToString(Integer) (Variables|Default|GetCurrentFloor))) :!label _label)
            (Utilities|FlowControl|DoOnce false) ; enters at Reset
          ))))
    (elif (== (Variables|Default|GetCurrentFloor) 0)
      (Variables|Default|Setb_Is_Up true)
      (CallFunction|MoveLift)
      (else
        (bind _output_get_3 (Variables|Default|SetCurrent (Transformation|GetActorLocation _self)))
        (for _array_element_2 (Variables|Default|GetFloors)
          (if (== (Variables|/Game/Lift/BP_TargetPoint.BP_TargetPoint_C|GetIndex _array_element_2) (- (Variables|Default|GetCurrentFloor) 1))
            (bind _output_get_4 (Variables|Default|SetTarget (Transformation|GetActorLocation _array_element_2)))))
        (bind _alpha_2 (Timeline|Timeline_1 PlayFromStart)
          (:Update
            (Transformation|SetActorLocation (Math|Vector|Lerp(Vector) _output_get_3 _output_get_4 _alpha_2) false false))
          (:Finished
            (Variables|Default|SetCurrentFloor (- (Variables|Default|GetCurrentFloor) 1))
            (goto _label)))))))

(event Custom|Call%20back
  (for _array_element (Variables|Default|GetFloors)
    (if (== (Variables|/Game/Lift/BP_TargetPoint.BP_TargetPoint_C|GetIndex _array_element) 0)
      (bind _output_get (Variables|Default|SetBase (Transformation|GetActorLocation _array_element)))
      (bind _alpha (Timeline|Timeline PlayFromStart)
        (:Update
          (Transformation|SetActorLocation (Math|Vector|Lerp(Vector) (Transformation|GetActorLocation) _output_get _alpha) false false))
        (:Finished
          (Variables|Default|SetCurrentFloor 0)
          (Variables|Default|Setb_Is_Up true))))))

(event EventBeginPlay
  (bind _outactors (Actor|GetAllActorsOfClass "/Game/Lift/BP_TargetPoint.BP_TargetPoint_C"))
  (Variables|Default|SetFloors _outactors))

(event EventInteract
  (Utilities|FlowControl|DoOnce false
    (:Completed
      (CallFunction|MoveLift))))

(fn ConstructionScript)

(fn IFGetHandSwayFloats
  (return 0.0 0.0 0.0))

(fn IFGetLeftHandSocketTransform
  (return ""))