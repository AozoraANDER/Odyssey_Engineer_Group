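; BP_LiftControl is an interactable control that calls the lift when used.
; Its Box overlap shows or hides the interact prompt, using TxtAction as the text, for the player character only.
; Interact finds the level's BP_Lift with GetActorOfClass and runs its CallBack, so it is not bound to a specific lift instance.
; The hand-sway and left-hand socket interface functions are unimplemented stubs.
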(event OnComponentBeginOverlap(Box)
  (params (OverlappedComponent :type Primitive%20Component%20Object%20Reference) (OtherActor :type Actor%20Object%20Reference) (OtherComp :type Primitive%20Component%20Object%20Reference) (OtherBodyIndex :type Integer) (bFromSweep :type Boolean) (SweepResult :type Hit%20Result%20Structure%20%28by%20ref%29))
  (bind _returnvalue (Game|GetPlayerCharacter 0))
  (if (== OtherActor _returnvalue)
    (Class|BIPlayerInterface|SetInteractableState(Message) _returnvalue true (Variables|Default|GetTxt_Action))))

(event OnComponentEndOverlap(Box)
  (params (OverlappedComponent :type Primitive%20Component%20Object%20Reference) (OtherActor :type Actor%20Object%20Reference) (OtherComp :type Primitive%20Component%20Object%20Reference) (OtherBodyIndex :type Integer))
  (bind _returnvalue (Game|GetPlayerCharacter 0))
  (if (== _returnvalue OtherActor)
    (Class|BIPlayerInterface|SetInteractableState(Message) _returnvalue false (Variables|Default|GetTxt_Action))))

(event EventBeginPlay)

(event Collision|EventActorBeginOverlap
  (params (OtherActor :type Actor%20Object%20Reference)))

(event EventTick
  (params (DeltaSeconds :type Float%20%28single-precision%29)))

(event EventInteract
  (bind _returnvalue (Actor|GetActorOfClass "/Game/Lift/BP_Lift.BP_Lift_C"))
  (Default|CallBack _returnvalue))

(fn ConstructionScript)

(fn IFGetHandSwayFloats
  (return 0.0 0.0 0.0))

(fn IFGetLeftHandSocketTransform
  (return ""))